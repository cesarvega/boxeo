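; RandomBP is a spawner that places BPTarget actors at random around the player.
; Tick passes through a six-second Delay into a loop that calls SpawnTarget about every second.
; SpawnTarget picks a point within the Box extent centered on the player, randomizes pitch and yaw, and skips spawns whose collision cannot be resolved.
; An unfinished audio frequency-spectrum branch, apparently for sound-driven spawning, is disconnected and never runs.
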(event EventBeginPlay)

(event EventTick
  (params (DeltaSeconds :type Float%20%28single-precision%29))
  (Utilities|FlowControl|Delay 6.0)
  ;[1 1 1] Respawn
  (CallFunction|SpawnTarget :!label _label)
  (Utilities|FlowControl|Delay 1.0)
  (goto _label))

(fn ConstructionScript)

(fn SpawnTarget
  ;[1 1 1] Seleccion de modelo y ubicarlo en la posicion
  (Game|SpawnActorfromClass "/Game/target22/BlueprintsTarget/BPTarget.BPTarget_C" (Math|Transform|MakeTransform (Math|Random|RandomPointinBoundingBox (Transformation|GetActorLocation (Game|GetPlayerCharacter 0)) (Variables|/Script/Engine.BoxComponent|GetBoxExtent (Variables|Default|GetBox))) (Math|Rotator|MakeRotator 0.0 (Math|Random|RandomFloatinRange 0.0 9e+01) (Math|Random|RandomFloatinRange -9e+01 9e+01)) "0.800000,0.800000,0.800000") "AdjustIfPossibleButDontSpawnIfColliding" 0 0))